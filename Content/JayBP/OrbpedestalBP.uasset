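; Pedestal actor that triggers the win screen once the player has picked up at least three gems.
; On any Box overlap it reads the gem count from JayGI, then creates the WinScreenHUD widget, plays a 2D sound and toggles off the FirstPersonCharacter's HUD.
; The overlap checks neither the overlapping actor nor repeat triggers.
; Its own Widget component is hidden at BeginPlay.
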(event `self.ReceiveBeginPlay`
  ;[1 1 1] Setting Win Text Off
  (`SceneComponent.SetVisibility` (`self.Widget`) false false))

(event `self.Box.OnComponentBeginOverlap`
  (params (OverlappedComponent :type "PrimitiveComponent Object Reference") (OtherActor :type "Actor Object Reference") (OtherComp :type "PrimitiveComponent Object Reference") (OtherBodyIndex :type Integer) (bFromSweep :type Boolean) (SweepResult :type "HitResult Structure (by ref)"))
  ;[1 1 1] Reading whether the player has all the collectibles and activating the "Win" text
  (bind _asjay_gi (cast `/Game/JayBP/JayGI` (`GameplayStatics.GetGameInstance`)))
  (if (>= (`/Game/JayBP/JayGI.GemsPickedUp` _asjay_gi) 3)
    (bind _returnvalue (`|CreateWidget` "/Game/JayWidgets/WinScreenHUD.WinScreenHUD_C"))
    (`UserWidget.AddToViewport` _returnvalue 0)
    (`GameplayStatics.PlaySound2D` "/Game/JayAudio/Electrical_Sweep-Sweeper-1760111493.Electrical_Sweep-Sweeper-1760111493" 1.0 1.0 0.0 null null)
    (`/Game/JayBP/FirstPersonCharacter.ToggleHudOff` (cast `/Game/JayBP/FirstPersonCharacter` (`GameplayStatics.GetPlayerCharacter` 0) :!pure true))))

(fn `UserConstructionScript`)